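; BP_Particle is a maths demo actor that moves its Particle component along parametric curves over time.
; Each tick feeds game time since creation into the Pikachu macro and sets the component's relative Y and Z from its X and Y, scaled by Size.
; Pikachu holds sums of sine and cosine harmonics.
; An unused StarMacro holds cubed sine and cosine terms, the form of a four-pointed astroid.
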(event EventBeginPlay)

(event Collision|EventActorBeginOverlap
  (params (OtherActor :type Actor%20Object%20Reference)))

(event EventTick
  (params (DeltaSeconds :type Float%20%28single-precision%29))
  (bind _returnvalue (Actor|GetGameTimeSinceCreation))
  (bind (_x _y) (Utilities|Pikachu _returnvalue))
  (Transformation|SetRelativeLocation (Variables|Default|GetParticle) (Math|Vector|MakeVector 0.0 (* _x (Variables|Default|GetSize)) (* _y (Variables|Default|GetSize))) false false))

(fn ConstructionScript)