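; BP_RotationArrow is an actor that the player rotates in fixed steps about its local X, Y and Z axes using quaternion math.
; BeginPlay adds the default Enhanced Input mapping context, and three rotation input actions each trigger one step on their axis.
; Each step hand-builds a half-angle quaternion from RotationAngle and post-multiplies the current rotation by it or its inverse, depending on the input sign.
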(event Input|EnhancedActionEvents|EnhancedInputActionIA_Rot_X
  (params (ActionValue :type Float%20%28double-precision%29) (ElapsedSeconds :type Float%20%28double-precision%29) (TriggeredSeconds :type Float%20%28double-precision%29) (InputAction :type Input%20Action%20Object%20Reference :default "/Game/ThirdPerson/Input/Actions/IA_Rot_X.IA_Rot_X"))
  (bind _returnvalue (Transformation|GetActorRotation))
  (bind _rotationangle (Variables|Default|GetRotationAngle))
  (bind _returnvalue_2 (Math|Conversions|ToQuaternion(Rotator) _returnvalue))
  (bind _returnvalue_3 (/ _rotationangle 2.0))
  (bind _returnvalue_4 (Math|Trig|Sin(Degrees) _returnvalue_3))
  (bind _returnvalue_5 (Math|Trig|Cos(Degrees) _returnvalue_3))
  (bind _returnvalue_6 (Class|KismetMathLibrary|MakeQuat _returnvalue_4 0.0 0.0 _returnvalue_5))
  (:Started
    (Transformation|SetActorRotation (Math|Rotator|SelectRotator (Class|KismetMathLibrary|QuatRotator (* _returnvalue_2 _returnvalue_6)) (Class|KismetMathLibrary|QuatRotator (* _returnvalue_2 (Class|KismetMathLibrary|QuatInversed _returnvalue_6))) (> ActionValue 0.0)))))

(event Input|EnhancedActionEvents|EnhancedInputActionIA_Rot_Y
  (params (ActionValue :type Float%20%28double-precision%29) (ElapsedSeconds :type Float%20%28double-precision%29) (TriggeredSeconds :type Float%20%28double-precision%29) (InputAction :type Input%20Action%20Object%20Reference :default "/Game/ThirdPerson/Input/Actions/IA_Rot_Y.IA_Rot_Y"))
  (bind _returnvalue (Transformation|GetActorRotation))
  (bind _rotationangle (Variables|Default|GetRotationAngle))
  (bind _returnvalue_2 (Math|Conversions|ToQuaternion(Rotator) _returnvalue))
  (bind _returnvalue_3 (/ _rotationangle 2.0))
  (bind _returnvalue_4 (Math|Trig|Sin(Degrees) _returnvalue_3))
  (bind _returnvalue_5 (Math|Trig|Cos(Degrees) _returnvalue_3))
  (bind _returnvalue_6 (Class|KismetMathLibrary|MakeQuat 0.0 _returnvalue_4 0.0 _returnvalue_5))
  (:Started
    (Transformation|SetActorRotation (Math|Rotator|SelectRotator (Class|KismetMathLibrary|QuatRotator (* _returnvalue_2 _returnvalue_6)) (Class|KismetMathLibrary|QuatRotator (* _returnvalue_2 (Class|KismetMathLibrary|QuatInversed _returnvalue_6))) (> ActionValue 0.0)))))

(event Input|EnhancedActionEvents|EnhancedInputActionIA_Rot_Z
  (params (ActionValue :type Float%20%28double-precision%29) (ElapsedSeconds :type Float%20%28double-precision%29) (TriggeredSeconds :type Float%20%28double-precision%29) (InputAction :type Input%20Action%20Object%20Reference :default "/Game/ThirdPerson/Input/Actions/IA_Rot_Z.IA_Rot_Z"))
  (bind _returnvalue (Transformation|GetActorRotation))
  (bind _rotationangle (Variables|Default|GetRotationAngle))
  (bind _returnvalue_2 (Math|Conversions|ToQuaternion(Rotator) _returnvalue))
  (bind _returnvalue_3 (/ _rotationangle 2.0))
  (bind _returnvalue_4 (Math|Trig|Sin(Degrees) _returnvalue_3))
  (bind _returnvalue_5 (Math|Trig|Cos(Degrees) _returnvalue_3))
  (bind _returnvalue_6 (Class|KismetMathLibrary|MakeQuat 0.0 0.0 _returnvalue_4 _returnvalue_5))
  (:Started
    (Transformation|SetActorRotation (Math|Rotator|SelectRotator (Class|KismetMathLibrary|QuatRotator (* _returnvalue_2 _returnvalue_6)) (Class|KismetMathLibrary|QuatRotator (* _returnvalue_2 (Class|KismetMathLibrary|QuatInversed _returnvalue_6))) (> ActionValue 0.0)))))

(event EventBeginPlay
  (bind _returnvalue (Game|GetPlayerController 0))
  (bind _returnvalue_2 (PlayerController|LocalPlayerSubsystems|GetEnhancedInputLocalPlayerSubsystem _returnvalue))
  (Utilities|IsValid _returnvalue_2
    (:Is%20Valid
      (Input|AddMappingContext _returnvalue_2 "/Game/ThirdPerson/Input/IMC_Default.IMC_Default" 0 "(bIgnoreAllPressedKeysUntilRelease=True,bForceImmediately=False,bNotifyUserSettings=False)"))))

(fn ConstructionScript)