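; BP_Generator is a procedural generation actor that lays out gray road cells in a cross from a starting position on BeginPlay.
; StartGeneration destroys stored cells, then CreateRoads spawns a seed cell and grows outward over a set number of iterations.
; Each pass spawns from the previous pass's cells: a directionless cell branches four ways, others continue straight, spaced by scaled cell size.
; Grid-spawning and random-material logic is present but never runs.
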(event Custom|StartGeneration
  (bind _cells (Variables|Default|GetCells))
  (for _array_element _cells
    (Actor|DestroyActor _array_element))
  (Utilities|Array|Clear _cells)
  (Utilities|Array|Clear (Variables|Default|GetLastIterCells))
  (CallFunction|CreateRoads))

(event Custom|CreateRoads
  (bind _cellscale (Variables|Default|GetCellScale))
  (bind _cellscale_2 (Variables|Default|GetCellScale))
  (bind _returnvalue (Game|SpawnActorfromClass "/Game/ProceduralGeneration/BP_BaseCell.BP_BaseCell_C" (Math|Transform|MakeTransform (Variables|Default|GetstartingPos) "0, 0, 0" (Math|Vector|MakeVector _cellscale _cellscale 1.0)) "Undefined" "MultiplyWithRoot" 0 "/Game/ProceduralGeneration/Materials/MI_Gray.MI_Gray" "NewEnumerator4" 0))
  (Utilities|Array|Add (Variables|Default|GetCells) _returnvalue)
  (Utilities|Array|Add (Variables|Default|GetnextIterCells) _returnvalue)
  (for _index (range 0 (Variables|Default|GetIterations))
    (Variables|Default|SetLastIterCells (Variables|Default|GetnextIterCells))
    (Utilities|Array|Clear (Variables|Default|GetnextIterCells))
    (for _array_element (Variables|Default|GetLastIterCells)
      (bind _output_get (Variables|Default|SetCurrentCell _array_element))
      (switch Utilities|FlowControl|Switch|SwitchonE_Direction (Variables|/Game/ProceduralGeneration/BP_BaseCell.BP_BaseCell_C|GetSpawnedDirection _output_get)
        (:NewEnumerator0
          (Utilities|FlowControl|Sequence
            (:then_0
              (Variables|Default|SetspawnPosMultiplier "0.000000,1.000000,0.000000" :!label _label)
              (Variables|Default|SetnextSpawnDirection "NewEnumerator0"))))
        (:NewEnumerator1
          (Utilities|FlowControl|Sequence
            (:then_0
              (Variables|Default|SetspawnPosMultiplier "0.000000,-1.000000,0.000000" :!label _label_2)
              (Variables|Default|SetnextSpawnDirection "NewEnumerator1"))))
        (:NewEnumerator2
          (Utilities|FlowControl|Sequence
            (:then_0
              (Variables|Default|SetspawnPosMultiplier "-1.000000,0.000000,0.000000" :!label _label_3)
              (Variables|Default|SetnextSpawnDirection "NewEnumerator2"))))
        (:NewEnumerator3
          (Utilities|FlowControl|Sequence
            (:then_0
              (Variables|Default|SetspawnPosMultiplier "1.000000,0.000000,0.000000" :!label _label_4)
              (Variables|Default|SetnextSpawnDirection "NewEnumerator3"))))
        (:NewEnumerator4
          (Utilities|FlowControl|Sequence
            (:then_0
              (goto _label))
            (:then_1
              (goto _label_2))
            (:then_2
              (goto _label_3))
            (:then_3
              (goto _label_4)))))
      (bind _returnvalue_2 (Game|SpawnActorfromClass "/Game/ProceduralGeneration/BP_BaseCell.BP_BaseCell_C" (Math|Transform|MakeTransform (+ (* (Variables|Default|GetspawnOffset) (Variables|Default|GetspawnPosMultiplier)) (Transformation|GetActorLocation (Variables|Default|GetCurrentCell))) "0, 0, 0" (Math|Vector|MakeVector _cellscale_2 _cellscale_2 1.0)) "Undefined" "MultiplyWithRoot" 0 "/Game/ProceduralGeneration/Materials/MI_Gray.MI_Gray" (Variables|Default|GetnextSpawnDirection) 0))
      (Utilities|Array|Add (Variables|Default|GetnextIterCells) _returnvalue_2))))

(event EventBeginPlay
  (bind _cellscale (Variables|Default|GetCellScale))
  (Variables|Default|SetspawnOffset (Math|Vector|MakeVector (* _cellscale (Variables|Default|GetbaseCellWidth)) (* _cellscale (Variables|Default|GetbaseCellHeight)) 0.0))
  (CallFunction|StartGeneration))

(fn ConstructionScript)